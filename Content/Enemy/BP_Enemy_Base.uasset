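; Base enemy Blueprint that chases player 0 and ends the game when it dies.
; Tick calls ChasePlayer every frame, which runs AI MoveTo on the player and also re-calls itself after a delay.
; SetHealth subtracts damage; once Tick sees Health depleted, it destroys the actor, shows the EndGame widget and pauses.
; A separate Attack event calls Play Montage on the mesh.
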(event Custom|ChasePlayer
  (AI|AIMoveTo self "0, 0, 0" (Game|GetPlayerCharacter 0) 5.0 false
    (:then
      (Utilities|FlowControl|Delay 2.0)
      (CallFunction|ChasePlayer))))

(event Custom|Attack
  (Animation|Montage|PlayMontage (Variables|Character|GetMesh) 0))

(event EventBeginPlay)

(event EventTick
  (params (DeltaSeconds :type Float%20%28single-precision%29))
  (CallFunction|ChasePlayer)
  (if (<= (Variables|Default|GetHealth) 0.0)
    (Actor|DestroyActor)
    (bind _returnvalue (Game|ConstructObjectfromClass "/Game/Blueprint/EndGame.EndGame_C"))
    (UserInterface|Viewport|AddtoViewport _returnvalue 0)
    (Game|SetGamePaused true)))

(fn ConstructionScript)

(fn GetHealth
  (return (Variables|Default|GetHealth)))

(fn SetHealth
  (params (Damage :type Float%20%28double-precision%29))
  (Variables|Default|SetHealth (- (Variables|Default|GetHealth) Damage)))